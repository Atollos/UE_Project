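; Player controller Blueprint that turns Enhanced Input into movement and crouching for TD_Character.
; BeginPlay adds the IMC_Default mapping context and caches the controlled pawn as TD_Character.
; IA_Move feeds the cached character right and forward input relative to control yaw.
; IA_Crouch re-casts the controlled pawn on each event, crouching on Started and uncrouching on Canceled, with no Completed handler.
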(event `self.ReceiveBeginPlay`
  (`EnhancedInputSubsystemInterface.AddMappingContext` (pcsubsystem `EnhancedInputLocalPlayerSubsystem` (`GameplayStatics.GetPlayerController` 0)) "/Game/Blueprints/Input/IMC_Default.IMC_Default" 0 (struct))
  (bind _astd_character (cast `/Game/Blueprints/TD_Character` (`self.K2_GetPawn`))))

(event `EnhancedInput|/Game/Blueprints/Input/IA_Move`
  (params (ActionValue :type "Vector2D Structure") (ElapsedSeconds :type "Float (double-precision)") (TriggeredSeconds :type "Float (double-precision)") (InputAction :type "InputAction Object Reference" :default "/Game/Blueprints/Input/IA_Move.IA_Move"))
  (bind (_returnvalue_roll _returnvalue_pitch _returnvalue_yaw) (`KismetMathLibrary.BreakRotator` (`self.GetControlRotation`)))
  (bind _returnvalue (`KismetMathLibrary.MakeRotator` 0.0 0.0 _returnvalue_yaw))
  (:`Triggered`
    (`|ExecutionSequence`
      (:`then_0`
        (`Pawn.AddMovementInput` (stale `self.ReceiveBeginPlay` _astd_character) (`KismetMathLibrary.GetRightVector` _returnvalue) ActionValue_X false))
      (:`then_1`
        (`Pawn.AddMovementInput` (stale `self.ReceiveBeginPlay` _astd_character) (`KismetMathLibrary.GetForwardVector` _returnvalue) ActionValue_Y false)))))

(event `EnhancedInput|/Game/Blueprints/Input/IA_Crouch`
  (params (ActionValue :type Boolean) (ElapsedSeconds :type "Float (double-precision)") (TriggeredSeconds :type "Float (double-precision)") (InputAction :type "InputAction Object Reference" :default "/Game/Blueprints/Input/IA_Crouch.IA_Crouch"))
  (bind _returnvalue (`self.K2_GetPawn`))
  (:`Started`
    (bind _astd_character (cast `/Game/Blueprints/TD_Character` _returnvalue))
    (`Character.Crouch` _astd_character))
  (:`Canceled`
    (bind _astd_character_2 (cast `/Game/Blueprints/TD_Character` _returnvalue))
    (`Character.UnCrouch` _astd_character_2)))

(fn `UserConstructionScript`)